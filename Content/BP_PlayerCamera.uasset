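; Player camera that pans, rotates and zooms on a spring arm, and sends click targets to the selected creature AI.
; Tick pans along one actor axis from screen-edge or key input, easing out on release, and pauses while rotating.
; Both mouse axes share one rotation handler driving actor yaw and clamped arm pitch.
; Left click traces under the cursor into SelectedCreatureAI; a test key starts the first BP_BotAI's turn.
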(event EventBeginPlay
  (Variables|Default|SetmoveDirection (Transformation|GetActorLocation)))

(event EventTick
  (params (DeltaSeconds :type Float%20%28single-precision%29))
  (bind _returnvalue (Transformation|GetActorLocation))
  (bind _returnvalue_2 (Game|GetPlayerController 0))
  (bind (_sizex _sizey) (HUD|GetViewportSize _returnvalue_2))
  (bind (_locationx _locationy) (Game|Player|GetMousePosition _returnvalue_2))
  ;[0.5725 1 0.6653 0.1] Camera Mouse Move
  (if (not (Variables|Default|GetcameraRotate))
    (Utilities|FlowControl|Sequence
      (:then_0
        (Variables|Default|SetmousePositionX (Math|Float|Truncate _locationx))
        (Variables|Default|SetmousePositionY (Math|Float|Truncate _locationy))
        (Variables|Default|SetviewportRight _sizex)
        (Variables|Default|SetviewportBot _sizey)
        (Utilities|FlowControl|Sequence
          (:then_0
            (if (or (Variables|Default|GetisMoveTop) (<= (Variables|Default|GetmousePositionY) (+ (Variables|Default|GetviewportTop) (Variables|Default|GetviewportBorder))))
              (Variables|Default|SetmoveDirection (Transformation|GetActorForwardVector))))
          (:then_1
            (if (or (Variables|Default|GetisMoveRight) (>= (Variables|Default|GetmousePositionX) (- (Variables|Default|GetviewportRight) (Variables|Default|GetviewportBorder))))
              (Variables|Default|SetmoveDirection (Transformation|GetActorRightVector))))
          (:then_2
            (if (or (Variables|Default|GetisMoveBot) (>= (Variables|Default|GetmousePositionY) (- (Variables|Default|GetviewportBot) (Variables|Default|GetviewportBorder))))
              (Variables|Default|SetmoveDirection (* (Transformation|GetActorForwardVector) -1.0))))
          (:then_3
            (if (or (Variables|Default|GetisMoveLeft) (<= (Variables|Default|GetmousePositionX) (+ (Variables|Default|GetviewportLeft) (Variables|Default|GetviewportBorder))))
              (Variables|Default|SetmoveDirection (* (Transformation|GetActorRightVector) -1.0)))))
        (if (Math|Boolean|ORBoolean (or (Variables|Default|GetisMoveTop) (<= (Variables|Default|GetmousePositionY) (+ (Variables|Default|GetviewportTop) (Variables|Default|GetviewportBorder)))) (or (Variables|Default|GetisMoveRight) (>= (Variables|Default|GetmousePositionX) (- (Variables|Default|GetviewportRight) (Variables|Default|GetviewportBorder)))) (or (Variables|Default|GetisMoveBot) (>= (Variables|Default|GetmousePositionY) (- (Variables|Default|GetviewportBot) (Variables|Default|GetviewportBorder)))) (or (Variables|Default|GetisMoveLeft) (<= (Variables|Default|GetmousePositionX) (+ (Variables|Default|GetviewportLeft) (Variables|Default|GetviewportBorder)))))
          (Variables|Default|SetcameraMoving true)
          (else
            (Variables|Default|SetcameraMoving false))))
      (:then_1
        (if (Variables|Default|GetcameraMoving)
          (bind _output_get (Variables|Default|SetcameraMoveSpeed (Math|Interpolation|FInterpTo 0.0 4e+01 DeltaSeconds 1e+01)))
          (Transformation|SetActorLocation (+ _returnvalue (* (Variables|Default|GetmoveDirection) _output_get)) false false)
          (else
            (bind _output_get_2 (Variables|Default|SetcameraMoveSpeed (Math|Interpolation|FInterpTo (Variables|Default|GetcameraMoveSpeed) 0.0 DeltaSeconds 1e+01)))
            (Transformation|SetActorLocation (+ _returnvalue (* (Variables|Default|GetmoveDirection) _output_get_2)) false false)))))))

(event Input|ActionEvents|InputActionCameraRotate
  (params (Key :type Key%20Structure))
  ;[0.5725 1 0.6653 0.1] Camera Rotate
  (:Pressed
    (Variables|Default|SetcameraRotate true))
  (:Released
    (Variables|Default|SetcameraRotate false)))

(event Input|ActionEvents|InputActionLMBClick
  (params (Key :type Key%20Structure))
  (bind _returnvalue (Game|GetPlayerController 0))
  (bind (_worldlocation _worlddirection) (Game|Player|ConvertMouseLocationToWorldSpace _returnvalue))
  ;[0.5725 1 0.6653 0.1] Left Mouse Click and Raycast
  (:Pressed
    (Utilities|IsValid (Variables|Default|GetselectedCreatureAI)
      (:Is%20Valid
        (bind _outhit (Collision|LineTraceByChannel _worldlocation (+ _worldlocation (* _worlddirection 1e+04)) "TraceTypeQuery1" false 0 "ForDuration"))
        (bind _output_get (Variables|Default|SetlineTraceLocation (.ImpactPoint (Collision|BreakHitResult _outhit))))
        (Variables|/Game/AI/BP_BotAI.BP_BotAI_C|SetmouseClicedLocation (Variables|Default|GetselectedCreatureAI) _output_get)))))

(event Input|ActionEvents|InputActionMoveCameraTop
  (params (Key :type Key%20Structure))
  ;[0.5725 1 0.6653 0.1] WASD input
  (:Pressed
    (Variables|Default|SetisMoveTop true))
  (:Released
    (Variables|Default|SetisMoveTop false)))

(event Input|ActionEvents|InputActionMoveCameraBot
  (params (Key :type Key%20Structure))
  ;[0.5725 1 0.6653 0.1] WASD input
  (:Pressed
    (Variables|Default|SetisMoveBot true))
  (:Released
    (Variables|Default|SetisMoveBot false)))

(event Input|ActionEvents|InputActionMoveCameraLeft
  (params (Key :type Key%20Structure))
  ;[0.5725 1 0.6653 0.1] WASD input
  (:Pressed
    (Variables|Default|SetisMoveLeft true))
  (:Released
    (Variables|Default|SetisMoveLeft false)))

(event Input|ActionEvents|InputActionMoveCameraRight
  (params (Key :type Key%20Structure))
  ;[0.5725 1 0.6653 0.1] WASD input
  (:Pressed
    (Variables|Default|SetisMoveRight true))
  (:Released
    (Variables|Default|SetisMoveRight false)))

(event Input|ActionEvents|InputActionTestKey
  (params (Key :type Key%20Structure))
  (:Pressed
    (bind _outactors (Actor|GetAllActorsOfClass "/Game/AI/BP_BotAI.BP_BotAI_C"))
    (Variables|/Game/AI/BP_BotAI.BP_BotAI_C|SetStartTurn (Utilities|Array|Get(acopy) _outactors) true)))

(event Input|AxisEvents|InputAxisCameraScroll
  (params (AxisValue :type Float%20%28single-precision%29))
  (bind _springarm (Variables|Default|GetSpringArm))
  ;[0.5725 1 0.6653 0.1] Camera Scroll
  (if (!= AxisValue 0.0)
    (if (<= (Variables|/Script/Engine.SpringArmComponent|GetTargetArmLength (Variables|Default|GetSpringArm)) (Variables|Default|GetminZoom))
      (Variables|/Script/Engine.SpringArmComponent|SetTargetArmLength _springarm (Variables|Default|GetminZoom))
      (if (not (< AxisValue 0.0))
        (Variables|/Script/Engine.SpringArmComponent|SetTargetArmLength _springarm (+ (Variables|/Script/Engine.SpringArmComponent|GetTargetArmLength (Variables|Default|GetSpringArm)) (* AxisValue (Variables|Default|GetcameraScrollSpeed))) :!label _label))
      (elif (>= (Variables|/Script/Engine.SpringArmComponent|GetTargetArmLength (Variables|Default|GetSpringArm)) (Variables|Default|GetmaxZoom))
        (Variables|/Script/Engine.SpringArmComponent|SetTargetArmLength _springarm (Variables|Default|GetmaxZoom))
        (if (not (> AxisValue 0.0))
          (goto _label))
        (else
          (goto _label))))))

(event Input|AxisEvents|InputAxisMouseAxisY
  (params (AxisValue :type Float%20%28single-precision%29))
  (bind _returnvalue (Transformation|GetActorRotation))
  (bind _springarm (Variables|Default|GetSpringArm))
  (bind _relativerotation (Variables|/Script/Engine.SceneComponent|GetRelativeRotation _springarm))
  ;[0.5725 1 0.6653 0.1] Camera Rotate
  (if (Variables|Default|GetcameraRotate)
    (Variables|Default|SetpitchRotationLimit (+ AxisValue (.pitch _relativerotation)))
    (Transformation|SetActorRotation (Math|Rotator|MakeRotator (.roll _returnvalue) (.pitch _returnvalue) (+ (stale Input|AxisEvents|InputAxisMouseAxisX AxisValue) (.yaw _returnvalue))))
    (if (> (Variables|Default|GetpitchRotationLimit) -1e+01)
      (Variables|Default|SetpitchRotationLimit -1e+01)
      (elif (< (Variables|Default|GetpitchRotationLimit) -8e+01)
        (Variables|Default|SetpitchRotationLimit -8e+01)))
    (Transformation|SetRelativeRotation _springarm (Math|Rotator|MakeRotator (.roll _relativerotation) (Variables|Default|GetpitchRotationLimit) (.yaw _relativerotation)) false false)))

(event Input|AxisEvents|InputAxisMouseAxisX
  (params (AxisValue :type Float%20%28single-precision%29))
  (bind _returnvalue (Transformation|GetActorRotation))
  (bind _springarm (Variables|Default|GetSpringArm))
  (bind _relativerotation (Variables|/Script/Engine.SceneComponent|GetRelativeRotation _springarm))
  ;[0.5725 1 0.6653 0.1] Camera Rotate
  (if (Variables|Default|GetcameraRotate)
    (Variables|Default|SetpitchRotationLimit (+ (stale Input|AxisEvents|InputAxisMouseAxisY AxisValue) (.pitch _relativerotation)))
    (Transformation|SetActorRotation (Math|Rotator|MakeRotator (.roll _returnvalue) (.pitch _returnvalue) (+ AxisValue (.yaw _returnvalue))))
    (if (> (Variables|Default|GetpitchRotationLimit) -1e+01)
      (Variables|Default|SetpitchRotationLimit -1e+01)
      (elif (< (Variables|Default|GetpitchRotationLimit) -8e+01)
        (Variables|Default|SetpitchRotationLimit -8e+01)))
    (Transformation|SetRelativeRotation _springarm (Math|Rotator|MakeRotator (.roll _relativerotation) (Variables|Default|GetpitchRotationLimit) (.yaw _relativerotation)) false false)))

(fn ConstructionScript)

(fn CameraMove
  (params (Direction :type Vector) (Delta%20Time :type Float%20%28single-precision%29) (CameraStartMove :type Boolean))
  (if CameraStartMove
    (Transformation|SetActorLocation (+ (Transformation|GetActorLocation) Direction) false false)
    (else
      (Transformation|SetActorLocation (Transformation|GetActorLocation) false false))))