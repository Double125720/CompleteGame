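; BP_PlayerManager handles player input for the creature whose turn it is in a turn-based battle.
; Tick fetches that creature from CPP_BattleManager and, while it is selected, previews the navmesh path to the cursor with debug lines and a decal.
; Clicking issues an AI move, gated by MoveEnd until it finishes or fails.
; It also handles deselection, ending turns and an F-key physics test on RifleIdle.
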(event Custom|End%20Turn%20Button
  (Class|CPPCreature|SetEndTurnState (Variables|Default|GetplayerCreature) true))

(event EventBeginPlay
  (Input|EnableInput (Game|GetPlayerController 0))
  (bind _asbp_player_camera (Utilities|Casting|CastToBP_PlayerCamera (Game|Player|GetPlayerPawn 0)))
  (Variables|Default|SetplayerCamera _asbp_player_camera))

(event EventTick
  (params (DeltaSeconds :type Float%20%28single-precision%29))
  (bind _returnvalue (Game|GetPlayerController 0))
  (bind _hitresult (Game|Player|GetHitResultUnderCursorbyChannel _returnvalue "TraceTypeQuery2" true))
  (bind _impactpoint (Collision|BreakHitResult _hitresult))
  (Utilities|FlowControl|Sequence
    (:then_0
      (bind _outactors (Actor|GetAllActorsOfClass "/Script/CompleteGame.CPP_BattleManager"))
      (bind _returnvalue_2 (Class|CPPBattleManager|GetCurrentTurnCreature (Utilities|Array|Get(acopy) _outactors)))
      (bind _asbp_bot_test (Utilities|Casting|CastToBP_BotTest _returnvalue_2))
      (Variables|Default|SetplayerCreature _asbp_bot_test))
    (:then_1
      (if (Variables|/Game/AI/BP_BotTest.BP_BotTest_C|GetSelected (Variables|Default|GetplayerCreature))
        (bind _returnvalue_3 (Class|NavigationSystem|FindPathtoLocationSynchronously (Transformation|GetActorLocation (Variables|Default|GetplayerCreature)) _impactpoint))
        (Transformation|SetWorldLocation (Variables|Default|GetDecal) _impactpoint false false)
        (for _index (range 0 (- (Utilities|Array|Length (Variables|/Script/Engine.NavigationPath|GetPathPoints _returnvalue_3)) 2))
          (Rendering|Debug|DrawDebugLine (Utilities|Array|Get(acopy) (Variables|/Script/Engine.NavigationPath|GetPathPoints _returnvalue_3) _index) (Utilities|Array|Get(acopy) (Variables|/Script/Engine.NavigationPath|GetPathPoints _returnvalue_3) (+ _index 1)) "(R=1.000000,G=0.009744,B=0.000000,A=1.000000)" 0.0 0.0)
          (Transformation|SetWorldLocation (Variables|Default|GetDecal) (Utilities|Array|Get(acopy) (Variables|/Script/Engine.NavigationPath|GetPathPoints _returnvalue_3) (+ _index 1)) false false))
        (else
          (Rendering|SetVisibility (Variables|Default|GetDecal) false false))))))

(event Input|ActionEvents|InputActionLMBClick
  (params (Key :type Key%20Structure))
  (bind _playercreature (Variables|Default|GetplayerCreature))
  (:Pressed
    (if (Variables|/Game/AI/BP_BotTest.BP_BotTest_C|GetSelected (Variables|Default|GetplayerCreature))
      (Rendering|SetVisibility (Variables|Default|GetDecal) true false)
      (if (Variables|Default|GetmoveEnd)
        (Variables|Default|SetmoveEnd false)
        (if (Variables|/Game/AI/BP_BotTest.BP_BotTest_C|GetSelected _playercreature)
          (AI|AIMoveTo (Variables|/Game/AI/BP_BotTest.BP_BotTest_C|GetRefBP_BotAI _playercreature) (.ImpactPoint (Collision|BreakHitResult (.HitResult (Game|Player|GetHitResultUnderCursorbyChannel (Game|GetPlayerController 0) "TraceTypeQuery2" true)))) 0 1.0 "Disable" "Default" true true
            (:OnRequestFailed
              _)
            (:OnMoveFinished
              _))
          (Variables|Default|SetmoveEnd true)))
      (else
        (Variables|Default|SetmoveEnd true)))))

(event Input|ActionEvents|InputActionDeselect
  (params (Key :type Key%20Structure))
  (bind _playercreature (Variables|Default|GetplayerCreature))
  (:Pressed
    (if (Variables|/Game/AI/BP_BotTest.BP_BotTest_C|GetSelected _playercreature)
      (Variables|/Game/AI/BP_BotTest.BP_BotTest_C|SetSelected _playercreature false))))

(event Input|KeyboardEvents|F
  (params (Key :type Key%20Structure))
  (bind _playercreature (Variables|Default|GetplayerCreature))
  (bind _rifle_idle (Variables|/Game/AI/BP_BotTest.BP_BotTest_C|GetRifle_Idle _playercreature))
  (:Pressed
    (Development|PrintString "f")
    (Audio|Components|Audio|Stop _rifle_idle)
    (Physics|SetSimulatePhysics _rifle_idle true))
  (:Released
    (Physics|SetSimulatePhysics _rifle_idle false)
    (Audio|Components|Audio|Play _rifle_idle true)))

(fn ConstructionScript)