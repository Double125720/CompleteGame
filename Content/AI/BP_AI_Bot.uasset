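; AI controller for a bot pawn that runs the BT_Bot behavior tree and handles turn waiting through the BB_Bot blackboard.
; On begin play it registers itself on BP_BotTest and stores the pawn's location as HomeLocation.
; Each tick it clears the player camera's selected creature AI and copies the clicked location to MoveLocation.
; StartTurn raises IsWait once through a DoOnce, which resets along with StartTurn when IsWait is false.
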(event EventBeginPlay
  (Utilities|FlowControl|Sequence
    (:then_0
      (bind _asbp_bot_test (Utilities|Casting|CastToBP_BotTest (Pawn|GetControlledPawn)))
      (Variables|/Game/AI/BP_BotTest.BP_BotTest_C|SetRefBP_BotAI _asbp_bot_test self))
    (:then_1
      (Class|AIController|UseBlackboard "/Game/AI/BB_BOt.BB_Bot")
      (AI|Components|Blackboard|SetValueasVector (AI|GetBlackboard self) (Variables|Default|GetHomeLocation) (Transformation|GetActorLocation (Pawn|GetControlledPawn)))
      (AI|RunBehaviorTree "/Game/AI/BT_Bot.BT_Bot"))))

(event EventTick
  (params (DeltaSeconds :type Float%20%28single-precision%29))
  (Utilities|FlowControl|Sequence
    (:then_0
      (bind _asbp_player_camera (Utilities|Casting|CastToBP_PlayerCamera (Game|Player|GetPlayerPawn 0)))
      (Variables|/Game/BP_PlayerCamera.BP_PlayerCamera_C|SetselectedCreatureAI _asbp_player_camera 0)
      (AI|Components|Blackboard|SetValueasVector (AI|GetBlackboard self) (Variables|Default|GetMoveLocation) (Variables|Default|GetmouseClicedLocation)))
    (:then_1
      (if (Variables|Default|GetStartTurn)
        (Utilities|FlowControl|DoOnce false :!label _label
          (:Completed
            (AI|Components|Blackboard|SetValueasBool (AI|GetBlackboard self) (Variables|Default|GetisWait) true)))))
    (:then_2
      (if (ScalableFloat|GetValueasBool (AI|GetBlackboard self) (Variables|Default|GetisWait))
        (Utilities|FlowControl|Delay 0.4)
        (if (stale _output_get)
          (Development|PrintString "Wait..."))
        (else
          (bind _output_get (Variables|Default|SetStartTurn false))
          (goto _label Reset))))))

(fn ConstructionScript)