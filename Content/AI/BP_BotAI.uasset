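; AI controller for a bot creature that moves to mouse-clicked locations in turns.
; On BeginPlay it stores the pawn's start as HomeLocation in BB_Bot and runs BT_Bot.
; Each tick it registers itself as the player camera's selected creature AI and copies the clicked location to MoveLocation.
; StartTurn raises IsWait once through a DoOnce, which resets along with StartTurn whenever IsWait is false.
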(event EventBeginPlay
  (Class|AIController|UseBlackboard "/Game/AI/BB_BOt.BB_Bot")
  (AI|Components|Blackboard|SetValueasVector (AI|GetBlackboard self) (Variables|Default|GetHomeLocation) (Transformation|GetActorLocation (Pawn|GetControlledPawn)))
  (AI|RunBehaviorTree "/Game/AI/BT_Bot.BT_Bot"))

(event EventTick
  (params (DeltaSeconds :type Float%20%28single-precision%29))
  (bind _self self)
  (Utilities|FlowControl|Sequence
    (:then_0
      (bind _asbp_player_camera (Utilities|Casting|CastToBP_PlayerCamera (Game|Player|GetPlayerPawn 0)))
      (Variables|/Game/BP_PlayerCamera.BP_PlayerCamera_C|SetselectedCreatureAI _asbp_player_camera _self)
      (AI|Components|Blackboard|SetValueasVector (AI|GetBlackboard _self) (Variables|Default|GetMoveLocation) (Variables|Default|GetmouseClicedLocation)))
    (:then_1
      (if (Variables|Default|GetStartTurn)
        (Utilities|FlowControl|DoOnce false :!label _label
          (:Completed
            (AI|Components|Blackboard|SetValueasBool (AI|GetBlackboard self) (Variables|Default|GetisWait) true)))))
    (:then_2
      (if (ScalableFloat|GetValueasBool (AI|GetBlackboard self) (Variables|Default|GetisWait))
        (Development|PrintString "Wait...")
        (else
          (Variables|Default|SetStartTurn false)
          (goto _label Reset))))))

(fn ConstructionScript)